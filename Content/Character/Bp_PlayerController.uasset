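; Player-driven pawn Blueprint, named Bp_PlayerController, that turns axis input into camera look and movement.
; Yaw and Pitch axes feed controller rotation, with pitch inverted.
; MoveForward and MoveRight add movement input along the actor's own forward and right vectors rather than the control rotation.
; A SpringArm is referenced but not adjusted, and the construction script is empty.
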(event Input|AxisEvents|InputAxisMoveForward
  (params (AxisValue :type Float%20%28single-precision%29))
  (Pawn|Input|AddMovementInput (Math|Vector|GetForwardVector (Transformation|GetActorRotation)) AxisValue false))

(event Input|AxisEvents|InputAxisMoveRight
  (params (AxisValue :type Float%20%28single-precision%29))
  (Pawn|Input|AddMovementInput (Math|Vector|GetRightVector (Transformation|GetActorRotation)) AxisValue false))

(event Input|AxisEvents|InputAxisYaw
  (params (AxisValue :type Float%20%28single-precision%29))
  (Pawn|Input|AddControllerYawInput AxisValue))

(event Input|AxisEvents|InputAxisPitch
  (params (AxisValue :type Float%20%28single-precision%29))
  (Variables|Default|SetSpringArm (Variables|Default|GetSpringArm))
  (Pawn|Input|AddControllerPitchInput (* AxisValue -1.0)))

(fn ConstructionScript)