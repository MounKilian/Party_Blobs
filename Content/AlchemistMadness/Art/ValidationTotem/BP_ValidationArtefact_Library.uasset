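; Validation artefact actor that animates the totem's three circle meshes and one orb with continuous relative rotation.
; Tick plays the ArtefactAnimations timeline, whose tracks, plus fixed offsets, set roll on circles one and three, pitch on circle two and yaw on the orb.
; The updates are nested: each rotation restarts another timeline from the start, and that timeline's update drives the next part while still reading ArtefactAnimations values.
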(event EventBeginPlay)

(event Collision|EventActorBeginOverlap
  (params (OtherActor :type Actor%20Object%20Reference)))

(event EventTick
  (params (DeltaSeconds :type Float%20%28single-precision%29))
  (bind (_direction _circle_01_rotation _circle_02_rotation _circle_03_rotation _orbe_rotation) (Timeline|Artefact%20Animations Play)
    (:Update
      (Transformation|SetRelativeRotation (Variables|Default|GetSM_ValidationArtefact_Circle_01) (Math|Rotator|MakeRotator (+ _circle_01_rotation -3.6e+02) 0.0 0.0) false false)
      (Timeline|Timeline_1 PlayFromStart
        (:Update
          (Transformation|SetRelativeRotation (Variables|Default|GetSM_ValidationArtefact_Circle_02) (Math|Rotator|MakeRotator 0.0 (+ _circle_02_rotation -3.6e+02) 0.0) false false)
          (Timeline|Timeline PlayFromStart
            (:Update
              (Transformation|SetRelativeRotation (Variables|Default|GetSM_ValidationArtefact_Circle_03) (Math|Rotator|MakeRotator (+ _circle_03_rotation -4.1e+02) 0.0 0.0) false false)
              (Timeline|Timeline_2 PlayFromStart
                (:Update
                  (Transformation|SetRelativeRotation (Variables|Default|GetSM_ValidationArtefact_Orbe_01) (Math|Rotator|MakeRotator 0.0 0.0 (+ _orbe_rotation -3.6e+02)) false false))))))))))

(fn ConstructionScript)