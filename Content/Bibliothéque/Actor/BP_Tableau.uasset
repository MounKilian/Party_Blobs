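; BP_Tableau is an interactive tableau in the library that cycles through three visual states, apparently as a puzzle piece.
; Overlapping its box enables player input and shows the PressE prompt; leaving reverses both.
; Each E press advances a looping MultiGate that swaps which of three static meshes is visible.
; SolutionTableau starts true and stays true only while the first mesh's state is active.
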(event OnComponentBeginOverlap(Box)
  (params (OverlappedComponent :type Primitive%20Component%20Object%20Reference) (OtherActor :type Actor%20Object%20Reference) (OtherComp :type Primitive%20Component%20Object%20Reference) (OtherBodyIndex :type Integer) (bFromSweep :type Boolean) (SweepResult :type Hit%20Result%20Structure%20%28by%20ref%29))
  (Input|EnableInput (Game|GetPlayerController 0))
  (Rendering|SetVisibility (Variables|Default|GetPress%20E) true false))

(event OnComponentEndOverlap(Box)
  (params (OverlappedComponent :type Primitive%20Component%20Object%20Reference) (OtherActor :type Actor%20Object%20Reference) (OtherComp :type Primitive%20Component%20Object%20Reference) (OtherBodyIndex :type Integer))
  (Input|DisableInput (Game|GetPlayerController 0))
  (Rendering|SetVisibility (Variables|Default|GetPress%20E) false false))

(event EventBeginPlay
  (Variables|Default|SetSolutionTableau true))

(event Input|KeyboardEvents|E
  (params (Key :type Key%20Structure :default "None"))
  (:Pressed
    (Utilities|FlowControl|MultiGate false true -1
      (:Out%200
        (Rendering|SetVisibility (Variables|Default|GetStaticMesh1) false false)
        (Rendering|SetVisibility (Variables|Default|GetStaticMesh2) true false)
        (Variables|Default|SetSolutionTableau false))
      (:Out%201
        (Rendering|SetVisibility (Variables|Default|GetStaticMesh2) false false)
        (Rendering|SetVisibility (Variables|Default|GetStaticMesh3) true false)
        (Variables|Default|SetSolutionTableau false))
      (:Out%202
        (Rendering|SetVisibility (Variables|Default|GetStaticMesh3) false false)
        (Rendering|SetVisibility (Variables|Default|GetStaticMesh1) true false)
        (Variables|Default|SetSolutionTableau true)))))

(fn ConstructionScript)