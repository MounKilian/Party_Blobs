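; Validation trigger for the tutorial alchemy puzzle, which opens the tutorial gate when solved.
; Overlapping its box enables input and shows a press-E prompt.
; Pressing E compares its Solution to the values on Bp_Tuto1, Bp_Tuto2 and Bp_Tuto3, found by class lookup.
; A full match opens BP_Gate_Tuto, and either outcome slides a success or error WB_Alchimie message on for a few seconds.
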(event OnComponentBeginOverlap(Box)
  (params (OverlappedComponent :type Primitive%20Component%20Object%20Reference) (OtherActor :type Actor%20Object%20Reference) (OtherComp :type Primitive%20Component%20Object%20Reference) (OtherBodyIndex :type Integer) (bFromSweep :type Boolean) (SweepResult :type Hit%20Result%20Structure%20%28by%20ref%29))
  (Input|EnableInput (Game|GetPlayerController 0))
  (Rendering|SetVisibility (Variables|Default|GetPress%20E) true false))

(event OnComponentEndOverlap(Box)
  (params (OverlappedComponent :type Primitive%20Component%20Object%20Reference) (OtherActor :type Actor%20Object%20Reference) (OtherComp :type Primitive%20Component%20Object%20Reference) (OtherBodyIndex :type Integer))
  (Input|DisableInput (Game|GetPlayerController 0))
  (Rendering|SetVisibility (Variables|Default|GetPress%20E) false false))

(event Custom|Open
  (params (Other%20Actor :type Actor%20Object%20Reference))
  (bind _asbp_gate_tuto (Utilities|Casting|CastToBP_Gate_Tuto Other%20Actor))
  (Default|Opening _asbp_gate_tuto))

(event Input|KeyboardEvents|E
  (params (Key :type Key%20Structure :default "None"))
  (:Pressed
    (bind _outactors (Actor|GetAllActorsOfClass "/Game/AlchemistMadness/Art/Entrance/Blueprints/Bp_Tuto1.Bp_Tuto1_C"))
    (if (== (Variables|Default|Getsolution) (Variables|/Game/AlchemistMadness/Art/Entrance/Blueprints/Bp_Tuto1.Bp_Tuto1_C|GetSolution1 (Utilities|Array|Get(acopy) _outactors)))
      (bind _outactors_2 (Actor|GetAllActorsOfClass "/Game/AlchemistMadness/Art/Entrance/Blueprints/Bp_Tuto2.Bp_Tuto2_C"))
      (if (== (Variables|/Game/AlchemistMadness/Art/Entrance/Blueprints/Bp_Tuto2.Bp_Tuto2_C|GetSolution2 (Utilities|Array|Get(acopy) _outactors_2)) (Variables|Default|Getsolution))
        (bind _outactors_3 (Actor|GetAllActorsOfClass "/Game/AlchemistMadness/Art/Entrance/Blueprints/Bp_Tuto3.Bp_Tuto3_C"))
        (if (== (Variables|/Game/AlchemistMadness/Art/Entrance/Blueprints/Bp_Tuto3.Bp_Tuto3_C|GetSolution3 (Utilities|Array|Get(acopy) _outactors_3)) (Variables|Default|Getsolution))
          (bind _outactors_4 (Actor|GetAllActorsOfClass "/Game/AlchemistMadness/Art/Entrance/Blueprints/BP_Gate_Tuto.BP_Gate_Tuto_C"))
          (CallFunction|Open (Utilities|Array|Get(acopy) _outactors_4))
          (bind _returnvalue (UserInterface|CreateWidget "/Game/Alchimie/WB_Alchimie.WB_Alchimie_C"))
          (UserInterface|Viewport|AddtoViewport _returnvalue 0)
          (bind _foundwidgets (Widget|GetAllWidgetsOfClass "/Game/Alchimie/WB_Alchimie.WB_Alchimie_C" true))
          (Default|SlideGoodon (Utilities|Array|Get(acopy) _foundwidgets))
          (Utilities|FlowControl|Delay 5.0)
          (Default|SlideGoodOff (Utilities|Array|Get(acopy) _foundwidgets))
          (else
            (bind _returnvalue_2 (UserInterface|CreateWidget "/Game/Alchimie/WB_Alchimie.WB_Alchimie_C"))
            (UserInterface|Viewport|AddtoViewport _returnvalue_2 0)
            (bind _foundwidgets_2 (Widget|GetAllWidgetsOfClass "/Game/Alchimie/WB_Alchimie.WB_Alchimie_C" true))
            (Default|SlideErroron (Utilities|Array|Get(acopy) _foundwidgets_2))
            (Utilities|FlowControl|Delay 5.0)
            (Default|SlideErrorOff (Utilities|Array|Get(acopy) _foundwidgets_2))))
        (else
          (bind _returnvalue_3 (UserInterface|CreateWidget "/Game/Alchimie/WB_Alchimie.WB_Alchimie_C"))
          (UserInterface|Viewport|AddtoViewport _returnvalue_3 0)
          (bind _foundwidgets_3 (Widget|GetAllWidgetsOfClass "/Game/Alchimie/WB_Alchimie.WB_Alchimie_C" true))
          (Default|SlideErroron (Utilities|Array|Get(acopy) _foundwidgets_3))
          (Utilities|FlowControl|Delay 5.0)
          (Default|SlideErrorOff (Utilities|Array|Get(acopy) _foundwidgets_3))))
      (else
        (bind _returnvalue_4 (UserInterface|CreateWidget "/Game/Alchimie/WB_Alchimie.WB_Alchimie_C"))
        (UserInterface|Viewport|AddtoViewport _returnvalue_4 0)
        (bind _foundwidgets_4 (Widget|GetAllWidgetsOfClass "/Game/Alchimie/WB_Alchimie.WB_Alchimie_C" true))
        (Default|SlideErroron (Utilities|Array|Get(acopy) _foundwidgets_4))
        (Utilities|FlowControl|Delay 5.0)
        (Default|SlideErrorOff (Utilities|Array|Get(acopy) _foundwidgets_4))))))

(fn ConstructionScript)