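; Library gate actor that sends the player to the Observatoire level when they enter its trigger.
; On overlap by Bp_PlayerController, it plays a 2D sound, shows a WB_Fade animation, waits briefly, then opens the level and removes the first WB_Inventory widget.
; A separate Opening event destroys the Door and FrameDoor components to clear the gate.
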(event OnComponentBeginOverlap(Trigger)
  (params (OverlappedComponent :type Primitive%20Component%20Object%20Reference) (OtherActor :type Actor%20Object%20Reference) (OtherComp :type Primitive%20Component%20Object%20Reference) (OtherBodyIndex :type Integer) (bFromSweep :type Boolean) (SweepResult :type Hit%20Result%20Structure%20%28by%20ref%29))
  (Utilities|Casting|CastToBp_PlayerController OtherActor)
  (Audio|PlaySound2D 0 1.0 1.0 0.0 0 0)
  (bind _returnvalue (UserInterface|CreateWidget "/Game/WB_Fade.WB_Fade_C"))
  (UserInterface|Viewport|AddtoViewport _returnvalue 0)
  (Default|FadeAnim _returnvalue)
  (Utilities|FlowControl|Delay 0.5)
  (Game|OpenLevel(byName) "Observatoire")
  (bind _foundwidgets (Widget|GetAllWidgetsOfClass "/Game/Bibliothéque/WB_Inventory.WB_Inventory_C" true))
  (Widget|RemovefromParent (Utilities|Array|Get(acopy) _foundwidgets)))

(event Custom|Opening
  (Components|DestroyComponent (Variables|Default|GetDoor))
  (Components|DestroyComponent (Variables|Default|GetFrameDoor)))

(fn ConstructionScript)