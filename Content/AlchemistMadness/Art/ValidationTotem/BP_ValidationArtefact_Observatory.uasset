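; Observatory validation artefact that checks the room's puzzles when the player presses E inside its trigger box, which also shows a prompt.
; It compares the first chest, grimoire, world map and telescope found by class against Solution in nested checks.
; A full match opens the observatory gate and slides in the WB_Alchimie success widget; any mismatch shows a timed WB_Observatoire error.
; Tick drives chained timelines that rotate the three rings and orb.
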(event OnComponentBeginOverlap(Box)
  (params (OverlappedComponent :type Primitive%20Component%20Object%20Reference) (OtherActor :type Actor%20Object%20Reference) (OtherComp :type Primitive%20Component%20Object%20Reference) (OtherBodyIndex :type Integer) (bFromSweep :type Boolean) (SweepResult :type Hit%20Result%20Structure%20%28by%20ref%29))
  (Input|EnableInput (Game|GetPlayerController 0))
  (Rendering|SetVisibility (Variables|Default|GetPress%20E) true false))

(event OnComponentEndOverlap(Box)
  (params (OverlappedComponent :type Primitive%20Component%20Object%20Reference) (OtherActor :type Actor%20Object%20Reference) (OtherComp :type Primitive%20Component%20Object%20Reference) (OtherBodyIndex :type Integer))
  (Input|DisableInput (Game|GetPlayerController 0))
  (Rendering|SetVisibility (Variables|Default|GetPress%20E) false false))

(event Custom|Open
  (params (Other%20Actor :type Actor%20Object%20Reference))
  (bind _asbp_gate_observatoire (Utilities|Casting|CastToBP_Gate_Observatoire Other%20Actor))
  (Default|Opening _asbp_gate_observatoire))

(event EventTick
  (params (DeltaSeconds :type Float%20%28single-precision%29))
  (bind (_direction _circle_01_rotation _circle_02_rotation _circle_03_rotation _orbe_rotation) (Timeline|Artefact%20Animations Play)
    (:Update
      (Transformation|SetRelativeRotation (Variables|Default|GetSM_ValidationArtefact_Circle_01) (Math|Rotator|MakeRotator (+ _circle_01_rotation -3.6e+02) 0.0 0.0) false false)
      (Timeline|Timeline_1 PlayFromStart
        (:Update
          (Transformation|SetRelativeRotation (Variables|Default|GetSM_ValidationArtefact_Circle_02) (Math|Rotator|MakeRotator 0.0 (+ _circle_02_rotation -3.6e+02) 0.0) false false)
          (Timeline|Timeline PlayFromStart
            (:Update
              (Transformation|SetRelativeRotation (Variables|Default|GetSM_ValidationArtefact_Circle_03) (Math|Rotator|MakeRotator (+ _circle_03_rotation -4.1e+02) 0.0 0.0) false false)
              (Timeline|Timeline_2 PlayFromStart
                (:Update
                  (Transformation|SetRelativeRotation (Variables|Default|GetSM_ValidationArtefact_Orbe_01) (Math|Rotator|MakeRotator 0.0 0.0 (+ _orbe_rotation -3.6e+02)) false false))))))))))

(event Input|KeyboardEvents|E
  (params (Key :type Key%20Structure :default "None"))
  (:Pressed
    (bind _outactors (Actor|GetAllActorsOfClass "/Game/Observatoire/Actor/Bp_Coffre.Bp_Coffre_C"))
    (if (== (Variables|/Game/Observatoire/Actor/Bp_Coffre.Bp_Coffre_C|GetSolutionCoffre (Utilities|Array|Get(acopy) _outactors)) (Variables|Default|Getsolution))
      (bind _outactors_2 (Actor|GetAllActorsOfClass "/Game/Observatoire/Actor/BP_Grimoire.BP_Grimoire_C"))
      (if (== (Variables|/Game/Observatoire/Actor/BP_Grimoire.BP_Grimoire_C|GetSolutionGrimoire (Utilities|Array|Get(acopy) _outactors_2)) (Variables|Default|Getsolution))
        (bind _outactors_3 (Actor|GetAllActorsOfClass "/Game/Observatoire/Actor/BP_MapMonde.BP_MapMonde_C"))
        (if (== (Variables|/Game/Observatoire/Actor/BP_MapMonde.BP_MapMonde_C|GetSolutionMapMonde (Utilities|Array|Get(acopy) _outactors_3)) (Variables|Default|Getsolution))
          (bind _outactors_4 (Actor|GetAllActorsOfClass "/Game/Observatoire/Actor/BP_Télescope.BP_Télescope_C"))
          (if (== (Variables|/Game/Observatoire/Actor/BP_Télescope.BP_Télescope_C|GetSolutionTelescope (Utilities|Array|Get(acopy) _outactors_4)) (Variables|Default|Getsolution))
            (bind _outactors_5 (Actor|GetAllActorsOfClass "/Game/Observatoire/Actor/BP_Gate_Observatoire.BP_Gate_Observatoire_C"))
            (CallFunction|Open (Utilities|Array|Get(acopy) _outactors_5))
            (bind _returnvalue (UserInterface|CreateWidget "/Game/Alchimie/WB_Alchimie.WB_Alchimie_C"))
            (UserInterface|Viewport|AddtoViewport _returnvalue 0)
            (bind _foundwidgets (Widget|GetAllWidgetsOfClass "/Game/Alchimie/WB_Alchimie.WB_Alchimie_C" true))
            (Default|SlideGoodon (Utilities|Array|Get(acopy) _foundwidgets))
            (Utilities|FlowControl|Delay 5.0)
            (Default|SlideGoodOff (Utilities|Array|Get(acopy) _foundwidgets))
            (else
              (bind _returnvalue_2 (UserInterface|CreateWidget "/Game/Observatoire/WB_Observatoire.WB_Observatoire_C"))
              (UserInterface|Viewport|AddtoViewport _returnvalue_2 0)
              (bind _foundwidgets_2 (Widget|GetAllWidgetsOfClass "/Game/Observatoire/WB_Observatoire.WB_Observatoire_C" true))
              (Default|SlideErroron (Utilities|Array|Get(acopy) _foundwidgets_2))
              (Utilities|FlowControl|Delay 5.0)
              (Default|SlideErrorOff (Utilities|Array|Get(acopy) _foundwidgets_2))))
          (else
            (bind _returnvalue_3 (UserInterface|CreateWidget "/Game/Observatoire/WB_Observatoire.WB_Observatoire_C"))
            (UserInterface|Viewport|AddtoViewport _returnvalue_3 0)
            (bind _foundwidgets_3 (Widget|GetAllWidgetsOfClass "/Game/Observatoire/WB_Observatoire.WB_Observatoire_C" true))
            (Default|SlideErroron (Utilities|Array|Get(acopy) _foundwidgets_3))
            (Utilities|FlowControl|Delay 5.0)
            (Default|SlideErrorOff (Utilities|Array|Get(acopy) _foundwidgets_3))))
        (else
          (bind _returnvalue_4 (UserInterface|CreateWidget "/Game/Observatoire/WB_Observatoire.WB_Observatoire_C"))
          (UserInterface|Viewport|AddtoViewport _returnvalue_4 0)
          (bind _foundwidgets_4 (Widget|GetAllWidgetsOfClass "/Game/Observatoire/WB_Observatoire.WB_Observatoire_C" true))
          (Default|SlideErroron (Utilities|Array|Get(acopy) _foundwidgets_4))
          (Utilities|FlowControl|Delay 5.0)
          (Default|SlideErrorOff (Utilities|Array|Get(acopy) _foundwidgets_4))))
      (else
        (bind _returnvalue_5 (UserInterface|CreateWidget "/Game/Observatoire/WB_Observatoire.WB_Observatoire_C"))
        (UserInterface|Viewport|AddtoViewport _returnvalue_5 0)
        (bind _foundwidgets_5 (Widget|GetAllWidgetsOfClass "/Game/Observatoire/WB_Observatoire.WB_Observatoire_C" true))
        (Default|SlideErroron (Utilities|Array|Get(acopy) _foundwidgets_5))
        (Utilities|FlowControl|Delay 5.0)
        (Default|SlideErrorOff (Utilities|Array|Get(acopy) _foundwidgets_5))))))

(fn ConstructionScript)