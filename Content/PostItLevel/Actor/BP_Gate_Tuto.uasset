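; BP_Gate_Tuto is a tutorial gate actor that opens its door and sends the player to the Observatoire level.
; An Opening event plays the door sound and drives a timeline that rotates the Door component around yaw.
; Overlapping the Trigger with a Bp_PlayerController actor shows a WB_Fade widget, plays its fade animation, then loads the level after a short delay.
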(event OnComponentBeginOverlap(Trigger)
  (params (OverlappedComponent :type Primitive%20Component%20Object%20Reference) (OtherActor :type Actor%20Object%20Reference) (OtherComp :type Primitive%20Component%20Object%20Reference) (OtherBodyIndex :type Integer) (bFromSweep :type Boolean) (SweepResult :type Hit%20Result%20Structure%20%28by%20ref%29))
  (Utilities|Casting|CastToBp_PlayerController OtherActor)
  (bind _returnvalue (UserInterface|CreateWidget "/Game/WB_Fade.WB_Fade_C"))
  (UserInterface|Viewport|AddtoViewport _returnvalue 0)
  (Default|FadeAnim _returnvalue)
  (Utilities|FlowControl|Delay 0.5)
  (Game|OpenLevel(byName) "Observatoire"))

(event Custom|Opening
  (Audio|PlaySound2D "/Game/sound/door_sound.door_sound" 1.0 1.0 0.0 0 0)
  (bind _zrotation (Timeline|DoorOpening Play)
    (:Update
      (Transformation|SetRelativeRotation (Variables|Default|GetDoor) (Math|Rotator|MakeRotator 0.0 0.0 _zrotation) false false))))

(fn ConstructionScript)